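; Enemy AI Blueprint that walks the character around a looping patrol route of four destinations, starting at BeginPlay.
; The patrol event sets a slow walk speed and uses AI MoveTo to reach the destination at the current index.
; On success it waits a random delay, calls patrol again, then increments the index, wrapping to zero.
; Failed moves have no handling.
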(event Custom|Patrol_Ai
  ;[0.15 0.15 0.15 0.5] Patrol
  (Variables|/Script/Engine.CharacterMovementComponent|SetMaxWalkSpeed (Variables|Character|GetCharacterMovement) 1.5e+02)
  (AI|AIMoveTo self (Utilities|Array|Get(acopy) (Variables|Default|GetPatrol_Destination) (Variables|Default|GetLocaitons)) 0 5.0 false
    (:OnSuccess
      (Utilities|FlowControl|Delay (Math|Random|RandomFloatinRange 1.0 5.0))
      (CallFunction|PatrolAi)
      (Math|Integer|IncrementInt (Variables|Default|GetLocaitons)
        (:%20%20
          (if (== (Variables|Default|GetLocaitons) 4)
            (Variables|Default|SetLocaitons 0)))))))

(event Collision|EventActorBeginOverlap
  (params (OtherActor :type Actor%20Object%20Reference)))

(event EventTick
  (params (DeltaSeconds :type Float%20%28single-precision%29)))

(event EventBeginPlay
  (CallFunction|PatrolAi))

(fn ConstructionScript)